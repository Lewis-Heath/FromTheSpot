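; Goalkeeper actor that dives toward a target location using physics and can be reset to its starting spot.
; It records its starting transform on BeginPlay.
; Dive applies a mesh impulse from the actor location toward the target, scaled by a clamped mapping of the supplied line length.
; Reset briefly turns off physics simulation to move the mesh back, with a yaw offset on the saved rotation.
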(event `self.ReceiveBeginPlay`
  (set `self.StartingPosition` (`self.K2_GetActorLocation`))
  (set `self.StartingRotation` (`self.K2_GetActorRotation`)))

(event `Reset`
  (bind _mesh (`self.Mesh`))
  (`PrimitiveComponent.SetSimulatePhysics` _mesh false)
  (`SceneComponent.K2_SetWorldLocationAndRotation` _mesh (`self.StartingPosition`) (`KismetMathLibrary.MakeRotator` (.roll (`self.StartingRotation`)) (.pitch (`self.StartingRotation`)) (+ (.yaw (`self.StartingRotation`)) -90.0)) false false)
  (`PrimitiveComponent.SetSimulatePhysics` _mesh true))

(event `Dive`
  (params (TargetLocation :type "Vector Structure") (LineLength :type "Float (double-precision)"))
  (`PrimitiveComponent.AddImpulse` (`self.Mesh`) (* (`KismetMathLibrary.GetDirectionUnitVector` (`self.K2_GetActorLocation`) TargetLocation) (* (`KismetMathLibrary.MapRangeClamped` LineLength 0.0 500.0 0.0 0.5) 100000.0)) "None" false))

(fn `UserConstructionScript`)