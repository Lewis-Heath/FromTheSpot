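; BP_FootballGoal is a football goal that detects whether a BP_Football scores or misses and reports the result to the HUD.
; A GoalLine overlap reports a goal, while four MissHitBox volumes around it each report a miss.
; Each overlap filters for the ball, casts the first player controller's GetHUD result to WBP_HUD, and calls UpdateNotify with true or false.
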(event `self.GoalLine.OnComponentBeginOverlap`
  (params (OverlappedComponent :type "PrimitiveComponent Object Reference") (OtherActor :type "Actor Object Reference") (OtherComp :type "PrimitiveComponent Object Reference") (OtherBodyIndex :type Integer) (bFromSweep :type Boolean) (SweepResult :type "HitResult Structure (by ref)"))
  (cast `/Game/Blueprints/BP_Football` OtherActor)
  (bind _aswbp_hud (cast `/Game/Blueprints/WBP_HUD` (`PlayerController.GetHUD` (`GameplayStatics.GetPlayerController` 0))))
  (`/Game/Blueprints/WBP_HUD.UpdateNotify` _aswbp_hud true))

(event `self.MissHitBox.OnComponentBeginOverlap`
  (params (OverlappedComponent :type "PrimitiveComponent Object Reference") (OtherActor :type "Actor Object Reference") (OtherComp :type "PrimitiveComponent Object Reference") (OtherBodyIndex :type Integer) (bFromSweep :type Boolean) (SweepResult :type "HitResult Structure (by ref)"))
  (cast `/Game/Blueprints/BP_Football` OtherActor)
  (bind _aswbp_hud (cast `/Game/Blueprints/WBP_HUD` (`PlayerController.GetHUD` (`GameplayStatics.GetPlayerController` 0))))
  (`/Game/Blueprints/WBP_HUD.UpdateNotify` _aswbp_hud false))

(event `self.MissHitBox1.OnComponentBeginOverlap`
  (params (OverlappedComponent :type "PrimitiveComponent Object Reference") (OtherActor :type "Actor Object Reference") (OtherComp :type "PrimitiveComponent Object Reference") (OtherBodyIndex :type Integer) (bFromSweep :type Boolean) (SweepResult :type "HitResult Structure (by ref)"))
  (cast `/Game/Blueprints/BP_Football` OtherActor)
  (bind _aswbp_hud (cast `/Game/Blueprints/WBP_HUD` (`PlayerController.GetHUD` (`GameplayStatics.GetPlayerController` 0))))
  (`/Game/Blueprints/WBP_HUD.UpdateNotify` _aswbp_hud false))

(event `self.MissHitBox2.OnComponentBeginOverlap`
  (params (OverlappedComponent :type "PrimitiveComponent Object Reference") (OtherActor :type "Actor Object Reference") (OtherComp :type "PrimitiveComponent Object Reference") (OtherBodyIndex :type Integer) (bFromSweep :type Boolean) (SweepResult :type "HitResult Structure (by ref)"))
  (cast `/Game/Blueprints/BP_Football` OtherActor)
  (bind _aswbp_hud (cast `/Game/Blueprints/WBP_HUD` (`PlayerController.GetHUD` (`GameplayStatics.GetPlayerController` 0))))
  (`/Game/Blueprints/WBP_HUD.UpdateNotify` _aswbp_hud false))

(event `self.MissHitBox3.OnComponentBeginOverlap`
  (params (OverlappedComponent :type "PrimitiveComponent Object Reference") (OtherActor :type "Actor Object Reference") (OtherComp :type "PrimitiveComponent Object Reference") (OtherBodyIndex :type Integer) (bFromSweep :type Boolean) (SweepResult :type "HitResult Structure (by ref)"))
  (cast `/Game/Blueprints/BP_Football` OtherActor)
  (bind _aswbp_hud (cast `/Game/Blueprints/WBP_HUD` (`PlayerController.GetHUD` (`GameplayStatics.GetPlayerController` 0))))
  (`/Game/Blueprints/WBP_HUD.UpdateNotify` _aswbp_hud false))

(fn `UserConstructionScript`)