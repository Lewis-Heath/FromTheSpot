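; Penalty-shootout goalkeeper that dives to a goal zone and saves or catches the ball.
; Dive waits on a timing-based delay, then uses that zone's data for montage, speed, glove hitbox radius and catch probability.
; Body and glove hits report saves to the game mode; gloves also roll once for a catch, swapping the real ball for a hand-attached dummy.
; Hitboxes follow mesh sockets, and kit material follows glove type.
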(event `self.BP_Dive`
  (params (DiveInfo :type "DivePointInfo Structure (by ref)") (TimingMultiplier :type "Float (single-precision)"))
  (bind (_animation _speed _gloveradius _catchprobability) (break `DiveAnimationInfo` (select `EGoalLocation` (`.GoalLocationType` (break `DivePointInfo` DiveInfo)) :`FAR_TOP_LEFT` (`self.FarTopLeftDive`) :`FAR_MIDDLE_LEFT` (`self.FarMiddleLeftDive`) :`FAR_BOTTOM_LEFT` (`self.FarBottomLeftDive`) :`MID_TOP_LEFT` (`self.MidTopLeftDive`) :`MID_MIDDLE_LEFT` (`self.MidMiddleLeftDive`) :`MID_BOTTOM_LEFT` (`self.MidBottomLeftDive`) :`CLOSE_TOP_LEFT` (`self.CloseTopLeftDive`) :`CLOSE_MIDDLE_LEFT` (`self.CloseMiddleLeftDive`) :`CLOSE_BOTTOM_LEFT` (`self.CloseBottomLeftDive`) :`MIDDLE_TOP` (`self.MiddleTopMiddleDive`) :`MIDDLE_MIDDLE` (`self.MiddleMiddleMiddleDive`) :`MIDDLE_BOTTOM` (`self.MiddleBottomMiddleDive`) :`FAR_TOP_RIGHT` (`self.FarTopRightDive`) :`FAR_MIDDLE_RIGHT` (`self.FarMiddleRightDive`) :`FAR_BOTTOM_RIGHT` (`self.FarBottomRightDive`) :`MID_TOP_RIGHT` (`self.MidTopRightDive`) :`MID_MIDDLE_RIGHT` (`self.MidMiddleRightDive`) :`MID_BOTTOM_RIGHT` (`self.MidBottomRightDive`) :`CLOSE_TOP_RIGHT` (`self.CloseTopRightDive`) :`CLOSE_MIDDLE_RIGHT` (`self.CloseMiddleRightDive`) :`CLOSE_BOTTOM_RIGHT` (`self.CloseBottomRightDive`))))
  (`KismetSystemLibrary.Delay` (`KismetMathLibrary.SelectFloat` 0.0 (`KismetMathLibrary.MapRangeUnclamped` TimingMultiplier 0.0 1.0 0.4) (<= TimingMultiplier 0.2)))
  (set `self.CurrentCatchProbability` _catchprobability)
  (`|PlayMontage` (`self.GoalkeeperMesh`) _animation _speed
    (:`then`
      (`SphereComponent.SetSphereRadius` (`self.LeftGloveHitBox`) _gloveradius true)
      (`SphereComponent.SetSphereRadius` (`self.RightGloveHitBox`) _gloveradius true))
    (:`OnCompleted`
      (`SphereComponent.SetSphereRadius` (`self.LeftGloveHitBox`) 32.0 true)
      (`SphereComponent.SetSphereRadius` (`self.RightGloveHitBox`) 32.0 true)
      (`SceneComponent.SetVisibility` (`self.Football`) false false)
      (set `self.bCatchDecisionMade` false)
      (set `self.CurrentCatchProbability` 0.0))))

(event `self.GoalkeeperMesh.OnComponentHit`
  (params (HitComponent :type "PrimitiveComponent Object Reference") (OtherActor :type "Actor Object Reference") (OtherComp :type "PrimitiveComponent Object Reference") (NormalImpulse :type "Vector Structure") (Hit :type "HitResult Structure (by ref)"))
  (cast `Football` OtherActor)
  (bind _asfrom_the_spot_game_mode_base (cast `FromTheSpotGameModeBase` (`GameplayStatics.GetGameMode`)))
  (`FromTheSpotGameModeBase.PenaltySaved` _asfrom_the_spot_game_mode_base))

(event `self.LeftGloveHitBox.OnComponentHit`
  (params (HitComponent :type "PrimitiveComponent Object Reference") (OtherActor :type "Actor Object Reference") (OtherComp :type "PrimitiveComponent Object Reference") (NormalImpulse :type "Vector Structure") (Hit :type "HitResult Structure (by ref)"))
  (bind _asfootball (cast `Football` OtherActor))
  (`self.TryCatchBall` _asfootball))

(event `self.RightGloveHitBox.OnComponentHit`
  (params (HitComponent :type "PrimitiveComponent Object Reference") (OtherActor :type "Actor Object Reference") (OtherComp :type "PrimitiveComponent Object Reference") (NormalImpulse :type "Vector Structure") (Hit :type "HitResult Structure (by ref)"))
  (bind _asfootball (cast `Football` OtherActor))
  (`self.TryCatchBall` _asfootball))

(event `self.BP_UpdateMaterial`
  (params (NewGlovesType :type "EGlovesType Enum" :default "NONE"))
  (bind _goalkeepermesh (`self.GoalkeeperMesh`))
  (`/Engine/EditorBlueprintResources/StandardMacros.IsValid` _goalkeepermesh
    (:`Is Valid`
      (`PrimitiveComponent.SetMaterial` _goalkeepermesh 0 (select `EGlovesType` NewGlovesType :`NONE` "/Game/Materials/Player/M_GoalkeeperKitGreyGloves.M_GoalkeeperKitGreyGloves" :`GREY` "/Game/Materials/Player/M_GoalkeeperKitGreyGloves.M_GoalkeeperKitGreyGloves" :`WHITE` "/Game/Materials/Player/M_GoalkeeperKitGreyGloves.M_GoalkeeperKitGreyGloves" :`BLUE` "/Game/Materials/Player/M_GoalkeeperKitBlueGloves.M_GoalkeeperKitBlueGloves" :`GREEN` "/Game/Materials/Player/M_GoalkeeperKitGreenGloves.M_GoalkeeperKitGreenGloves" :`RED` "/Game/Materials/Player/M_GoalkeeperKitRedGloves.M_GoalkeeperKitRedGloves" :`YELLOW` "/Game/Materials/Player/M_GoalkeeperKitYellowGloves.M_GoalkeeperKitYellowGloves" :!type "Material Object Reference")))))

(fn `GetSoundVolumeMultiplier`
  (params (TypeIndex :type Integer) (BaseVolumeMultiplier :type "Float (double-precision)"))
  (returns (FinalVolumeMultiplier :type "Float (double-precision)"))
  (locals (OutVolumeMultiplier :type "Float (double-precision)"))
  (bind _asfrom_the_spot_game_instance (cast `FromTheSpotGameInstance` (`GameplayStatics.GetGameInstance`)))
  (bind _returnvalue (`FromTheSpotGameInstance.GetMatchVolumes` _asfrom_the_spot_game_instance))
  (return (* (* (`local.BaseVolumeMultiplier`) (`|GetArrayItem` _returnvalue)) (`|GetArrayItem` _returnvalue TypeIndex))))

(fn `TryCatchBall`
  (params (Ball :type "Football Object Reference"))
  (bind _footballmesh (`Football.FootballMesh` (`local.Ball`)))
  (`/Engine/EditorBlueprintResources/StandardMacros.IsValid` Ball
    (:`Is Valid`
      (if (not (`self.bCatchDecisionMade`))
        (bind _asfrom_the_spot_game_mode_base (cast `FromTheSpotGameModeBase` (`GameplayStatics.GetGameMode`)))
        (`FromTheSpotGameModeBase.PenaltySaved` _asfrom_the_spot_game_mode_base)
        (`GameplayStatics.PlaySoundAtLocation` (`KismetArrayLibrary.Array_Random` (`self.CrowdCheeringSounds`)) (`self.K2_GetActorLocation` self) (struct) (`self.GetSoundVolumeMultiplier` 3 0.5) 1.0 0.0 null null null null)
        (if (`KismetMathLibrary.RandomBoolWithWeight` (`self.CurrentCatchProbability`))
          (`SceneComponent.SetVisibility` (`self.Football`) true false)
          (`SceneComponent.SetVisibility` _footballmesh false false)
          (`PrimitiveComponent.SetSimulatePhysics` _footballmesh false)
          (`PrimitiveComponent.SetCollisionEnabled` _footballmesh "NoCollision")
          (bind _asfrom_the_spot_game_mode_base_2 (cast `FromTheSpotGameModeBase` (`GameplayStatics.GetGameMode`)))
          (`FromTheSpotGameModeBase.GoalMissed` _asfrom_the_spot_game_mode_base_2)
          (set `self.bCatchDecisionMade` true)
          (else
            (set `self.bCatchDecisionMade` true)))))))

(fn `UserConstructionScript`
  (`SceneComponent.K2_AttachToComponent` (`self.LeftGloveHitBox`) (`self.GoalkeeperMesh`) "LeftHand" "KeepRelative" "KeepRelative" "KeepRelative" true)
  (`SceneComponent.K2_AttachToComponent` (`self.RightGloveHitBox`) (`self.GoalkeeperMesh`) "RightHand" "KeepRelative" "KeepRelative" "KeepRelative" true)
  (`SceneComponent.K2_AttachToComponent` (`self.RightFootHitBox`) (`self.GoalkeeperMesh`) "RightFoot" "KeepRelative" "KeepRelative" "KeepRelative" true)
  (`SceneComponent.K2_AttachToComponent` (`self.Football`) (`self.GoalkeeperMesh`) "LeftHand" "KeepRelative" "KeepRelative" "KeepRelative" true))