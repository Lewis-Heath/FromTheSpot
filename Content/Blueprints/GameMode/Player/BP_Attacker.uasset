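; Player attacker for a penalty shootout game, handling the kick sequence, touch input and the follow camera.
; Match state changes pick an attack, defend or interaction camera point, and Tick linearly blends the camera's relative transform toward it.
; TakePenalty plays the kick montage in slow motion until completion; its notify tells the game mode to take the penalty and moves the camera to a second interaction point.
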(event `self.ReceiveBeginPlay`
  (bind _cameraattackpoint (`self.CameraAttackPoint`))
  (bind _relativelocation (`SceneComponent.RelativeLocation` _cameraattackpoint))
  (set `self.CameraStartingLocation` _relativelocation)
  (set `self.CameraTargetLocation` _relativelocation)
  (bind _output_get (set `self.CameraStartingRotation` (`SceneComponent.RelativeRotation` _cameraattackpoint)))
  (set `self.CameraTargetRotation` _output_get)
  (set `self.CurrentInterpAmount` 1.0))

(event `self.MatchStateStarted`
  (params (NewMatchState :type "EMatchState Enum" :default "NONE"))
  (switch `EMatchState` NewMatchState
    (:`ATTACK`
      (`self.UpdateCameraLerpTarget` (`self.CameraAttackPoint`) 2.0))
    (:`DEFEND`
      (`self.UpdateCameraLerpTarget` (`self.CameraDefendPoint`) 2.0))
    (:`INTERACTION`
      (`self.UpdateCameraLerpTarget` (`self.CameraInteractionPoint`) 2.0))))

(event `self.ReceiveTick`
  (params (DeltaSeconds :type "Float (single-precision)"))
  (`self.LerpCamera` DeltaSeconds))

(event `self.TakePenalty`
  (`GameplayStatics.PlaySound2D` "/Engine/VREditor/Sounds/UI/Enter_Simulate.Enter_Simulate" 1.0 1.0 0.0 null null)
  (`|PlayMontage` (`self.Mesh`) "/Game/Animations/Player/Attacker/AM_PenaltyKick.AM_PenaltyKick"
    (:`then`
      (`GameplayStatics.SetGlobalTimeDilation` 0.25))
    (:`OnCompleted`
      (`GameplayStatics.SetGlobalTimeDilation` 1.0))
    (:`OnNotifyBegin`
      (bind _asfrom_the_spot_game_mode_base (cast `FromTheSpotGameModeBase` (`GameplayStatics.GetGameMode`)))
      (`FromTheSpotGameModeBase.TakePenalty` _asfrom_the_spot_game_mode_base)
      (`self.UpdateCameraLerpTarget` (`self.CameraInteractionPoint2`) 4.0))))

(event `InputTouch`
  (params (Location :type "Vector Structure") (FingerIndex :type "ETouchIndex Enum"))
  (:`Pressed`
    (`self.TouchPressed` Location))
  (:`Released`
    (`self.TouchReleased` Location))
  (:`Moved`
    (`self.TouchMoved` Location)))

(fn `LerpCamera`
  (params (DeltaTime :type "Float (double-precision)"))
  (set `self.CurrentInterpAmount` (`KismetMathLibrary.FClamp` (+ (* DeltaTime (`self.InterpSpeed`)) (`self.CurrentInterpAmount`))))
  (`SceneComponent.K2_SetRelativeLocation` (`self.FollowCamera`) (`KismetMathLibrary.VLerp` (`self.CameraStartingLocation`) (`self.CameraTargetLocation`) (`self.CurrentInterpAmount`)) false false)
  (`SceneComponent.K2_SetRelativeRotation` (`self.FollowCamera`) (`KismetMathLibrary.RLerp` (`self.CameraStartingRotation`) (`self.CameraTargetRotation`) (`self.CurrentInterpAmount`)) false false))

(fn `UpdateCameraLerpTarget`
  (params (TargetPoint :type "SceneComponent Object Reference") (Speed :type "Float (double-precision)"))
  (bind _followcamera (`self.FollowCamera`))
  (set `self.CameraStartingLocation` (`SceneComponent.RelativeLocation` _followcamera))
  (set `self.CameraStartingRotation` (`SceneComponent.RelativeRotation` _followcamera))
  (set `self.CameraTargetLocation` (`SceneComponent.RelativeLocation` TargetPoint))
  (set `self.CameraTargetRotation` (`SceneComponent.RelativeRotation` TargetPoint))
  (set `self.CurrentInterpAmount` 0.0)
  (set `self.InterpSpeed` Speed))

(fn `UserConstructionScript`)