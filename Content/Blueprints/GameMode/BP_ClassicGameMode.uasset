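; Classic game mode Blueprint that folds end-of-match player stats into the persistent save.
; When end-match data updates, it loads the existing Save1 slot as BP_SaveData, adds the player's goals and saves to the stored totals, increments matches played, and writes it back.
; If no save exists, nothing is recorded, as this graph never creates one.
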(event `self.UpdateEndMatchData`
  (bind _returnvalue (`GameplayStatics.DoesSaveGameExist` "Save1"))
  (if _returnvalue
    (bind _returnvalue_2 (`GameplayStatics.LoadGameFromSlot` "Save1"))
    (bind _asbp_save_data (cast `/Game/Blueprints/GameMode/BP_SaveData` _returnvalue_2))
    (bind _output_get (set `self.SaveData` _asbp_save_data))
    (set `/Game/Blueprints/GameMode/BP_SaveData.GoalsScored` (+ (`self.PlayerGoalsScored`) (`/Game/Blueprints/GameMode/BP_SaveData.GoalsScored` _asbp_save_data)) _output_get)
    (set `/Game/Blueprints/GameMode/BP_SaveData.SavesMade` (+ (`self.PlayerSavesMade`) (`/Game/Blueprints/GameMode/BP_SaveData.SavesMade` _asbp_save_data)) _output_get)
    (set `/Game/Blueprints/GameMode/BP_SaveData.MatchesPlayed` (+ 1 (`/Game/Blueprints/GameMode/BP_SaveData.MatchesPlayed` _asbp_save_data)) _output_get)
    (`GameplayStatics.SaveGameToSlot` (`self.SaveData`) "Save1")))

(fn `UserConstructionScript`)