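; Football goal actor for a spot-kick game that reports scored and missed shots to the game mode.
; A BP_Football overlapping the goal line calls GoalScored on FromTheSpotGameModeBase, while overlapping any of four surrounding miss hit boxes calls GoalMissed.
; On BeginPlay it fills a DivePoints array that tags target points by goal location, covering only right-side and bottom positions.
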(event `self.ReceiveBeginPlay`
  (`KismetArrayLibrary.Array_Add` (`self.DivePoints`) (make `DivePointInfo` "FAR_TOP_RIGHT" (`self.TopRight`)))
  (`KismetArrayLibrary.Array_Add` (`self.DivePoints`) (make `DivePointInfo` "FAR_MIDDLE_RIGHT" (`self.MiddleRight`)))
  (`KismetArrayLibrary.Array_Add` (`self.DivePoints`) (make `DivePointInfo` "FAR_BOTTOM_RIGHT" (`self.BottomRight`)))
  (`KismetArrayLibrary.Array_Add` (`self.DivePoints`) (make `DivePointInfo` "MID_TOP_RIGHT" (`self.TopRight2`)))
  (`KismetArrayLibrary.Array_Add` (`self.DivePoints`) (make `DivePointInfo` "MID_MIDDLE_RIGHT" (`self.MiddleRight2`)))
  (`KismetArrayLibrary.Array_Add` (`self.DivePoints`) (make `DivePointInfo` "MID_BOTTOM_RIGHT" (`self.BottomRight2`)))
  (`KismetArrayLibrary.Array_Add` (`self.DivePoints`) (make `DivePointInfo` "CLOSE_TOP_RIGHT" (`self.TopRight3`)))
  (`KismetArrayLibrary.Array_Add` (`self.DivePoints`) (make `DivePointInfo` "CLOSE_MIDDLE_RIGHT" (`self.MiddleRight3`)))
  (`KismetArrayLibrary.Array_Add` (`self.DivePoints`) (make `DivePointInfo` "CLOSE_BOTTOM_RIGHT" (`self.BottomRight3`)))
  (`KismetArrayLibrary.Array_Add` (`self.DivePoints`) (make `DivePointInfo` "MIDDLE_BOTTOM" (`self.BottomMiddle`))))

(event `self.GoalLine.OnComponentBeginOverlap`
  (params (OverlappedComponent :type "PrimitiveComponent Object Reference") (OtherActor :type "Actor Object Reference") (OtherComp :type "PrimitiveComponent Object Reference") (OtherBodyIndex :type Integer) (bFromSweep :type Boolean) (SweepResult :type "HitResult Structure (by ref)"))
  (cast `/Game/Blueprints/GameMode/Football/BP_Football` OtherActor)
  (bind _asfrom_the_spot_game_mode_base (cast `FromTheSpotGameModeBase` (`GameplayStatics.GetGameMode`)))
  (`FromTheSpotGameModeBase.GoalScored` _asfrom_the_spot_game_mode_base))

(event `self.MissHitBox.OnComponentBeginOverlap`
  (params (OverlappedComponent :type "PrimitiveComponent Object Reference") (OtherActor :type "Actor Object Reference") (OtherComp :type "PrimitiveComponent Object Reference") (OtherBodyIndex :type Integer) (bFromSweep :type Boolean) (SweepResult :type "HitResult Structure (by ref)"))
  (cast `/Game/Blueprints/GameMode/Football/BP_Football` OtherActor)
  (bind _asfrom_the_spot_game_mode_base (cast `FromTheSpotGameModeBase` (`GameplayStatics.GetGameMode`)))
  (`FromTheSpotGameModeBase.GoalMissed` _asfrom_the_spot_game_mode_base))

(event `self.MissHitBox1.OnComponentBeginOverlap`
  (params (OverlappedComponent :type "PrimitiveComponent Object Reference") (OtherActor :type "Actor Object Reference") (OtherComp :type "PrimitiveComponent Object Reference") (OtherBodyIndex :type Integer) (bFromSweep :type Boolean) (SweepResult :type "HitResult Structure (by ref)"))
  (cast `/Game/Blueprints/GameMode/Football/BP_Football` OtherActor)
  (bind _asfrom_the_spot_game_mode_base (cast `FromTheSpotGameModeBase` (`GameplayStatics.GetGameMode`)))
  (`FromTheSpotGameModeBase.GoalMissed` _asfrom_the_spot_game_mode_base))

(event `self.MissHitBox2.OnComponentBeginOverlap`
  (params (OverlappedComponent :type "PrimitiveComponent Object Reference") (OtherActor :type "Actor Object Reference") (OtherComp :type "PrimitiveComponent Object Reference") (OtherBodyIndex :type Integer) (bFromSweep :type Boolean) (SweepResult :type "HitResult Structure (by ref)"))
  (cast `/Game/Blueprints/GameMode/Football/BP_Football` OtherActor)
  (bind _asfrom_the_spot_game_mode_base (cast `FromTheSpotGameModeBase` (`GameplayStatics.GetGameMode`)))
  (`FromTheSpotGameModeBase.GoalMissed` _asfrom_the_spot_game_mode_base))

(event `self.MissHitBox3.OnComponentBeginOverlap`
  (params (OverlappedComponent :type "PrimitiveComponent Object Reference") (OtherActor :type "Actor Object Reference") (OtherComp :type "PrimitiveComponent Object Reference") (OtherBodyIndex :type Integer) (bFromSweep :type Boolean) (SweepResult :type "HitResult Structure (by ref)"))
  (cast `/Game/Blueprints/GameMode/Football/BP_Football` OtherActor)
  (bind _asfrom_the_spot_game_mode_base (cast `FromTheSpotGameModeBase` (`GameplayStatics.GetGameMode`)))
  (`FromTheSpotGameModeBase.GoalMissed` _asfrom_the_spot_game_mode_base))

(fn `UserConstructionScript`)