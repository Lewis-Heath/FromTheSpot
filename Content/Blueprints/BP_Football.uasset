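; BP_Football is a physics-driven football that is shot toward a target location and can be reset to its starting position.
; ShootBall turns a timing value into a clamped force along the direction to the target, penalizing any timing short of a perfect 1.0.
; Hits on net components of BP_FootballGoal sharply damp the ball's velocity.
; Reset briefly disables physics simulation to move the mesh back to its spawn location.
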(event `self.ReceiveBeginPlay`
  (set `self.StartingPosition` (`self.K2_GetActorLocation`)))

(event `Reset`
  (bind _mesh (`self.Mesh`))
  (`PrimitiveComponent.SetSimulatePhysics` _mesh false)
  (`SceneComponent.K2_SetWorldLocation` _mesh (`self.StartingPosition`) false false)
  (`PrimitiveComponent.SetSimulatePhysics` _mesh true))

(event `ShootBall`
  (params (TargetLocation :type "Vector Structure") (TimingAmount :type "Float (double-precision)"))
  (bind _returnvalue (- TimingAmount 0.2))
  (set `self.PowerMultiplier` 0.0)
  (if (!= TimingAmount 1.0)
    (set `self.PowerMultiplier` (* (`KismetMathLibrary.MapRangeClamped` (`KismetMathLibrary.SelectFloat` 0.0 _returnvalue (< _returnvalue 0.0)) 0.0 1.0 0.2 1.9) 100000.0))
    (else
      (set `self.PowerMultiplier` (* (`KismetMathLibrary.MapRangeClamped` TimingAmount 0.0 1.0 0.2 1.9) 100000.0))))
  (`PrimitiveComponent.AddForce` (`self.Mesh`) (* (`KismetMathLibrary.GetDirectionUnitVector` (`self.K2_GetActorLocation`) TargetLocation) (`self.PowerMultiplier`)) "None" false))

(event `self.Mesh.OnComponentHit`
  (params (HitComponent :type "PrimitiveComponent Object Reference") (OtherActor :type "Actor Object Reference") (OtherComp :type "PrimitiveComponent Object Reference") (NormalImpulse :type "Vector Structure") (Hit :type "HitResult Structure (by ref)"))
  (bind _mesh (`self.Mesh`))
  (cast `/Game/Blueprints/BP_FootballGoal` OtherActor)
  (if (`KismetStringLibrary.Contains` (`KismetSystemLibrary.GetDisplayName` OtherComp) "Net")
    (bind _returnvalue (`PrimitiveComponent.GetPhysicsLinearVelocity` _mesh "None"))
    (`PrimitiveComponent.SetAllPhysicsLinearVelocity` _mesh (* _returnvalue 0.1) false)))

(fn `UserConstructionScript`)